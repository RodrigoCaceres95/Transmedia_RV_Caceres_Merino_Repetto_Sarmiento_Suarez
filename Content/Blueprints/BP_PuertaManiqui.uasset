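; BP_PuertaManiqui is a marble door that slides upward when its AbrirPuertaPorManiquis event is called, apparently by a mannequin-related trigger elsewhere.
; BeginPlay caches the mesh's closed relative location.
; The event checks the Abierta and Bloqueo flags, then plays a timeline that lerps the mesh up by AlturaApertura.
; The graph never sets either flag and has no closing logic.
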(event Custom|AbrirPuertaPorManiquis
  (bind _poscerrada (Variables|Default|GetposCerrada))
  (if (and (not (Variables|Default|Getabierta)) (not (Variables|Default|Getbloqueo)))
    (bind _apertura (Timeline|TLPuerta PlayFromStart)
      (:Update
        (Transformation|SetRelativeLocation (Variables|Default|GetSM_puerta_marmol) (Math|Vector|Lerp(Vector) _poscerrada (+ _poscerrada (Math|Vector|MakeVector 0.0 0.0 (Variables|Default|GetAlturaApertura))) _apertura) false false)))))

(event Collision|EventActorBeginOverlap
  (params (OtherActor :type Actor%20Object%20Reference)))

(event EventTick
  (params (DeltaSeconds :type Float%20%28single-precision%29)))

(event EventBeginPlay
  (Variables|Default|SetposCerrada (Variables|/Script/Engine.SceneComponent|GetRelativeLocation (Variables|Default|GetSM_puerta_marmol))))

(fn ConstructionScript)