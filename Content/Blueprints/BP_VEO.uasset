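; BP_VEO handles the VEO robot's exit from a chest through the SalirDelCofre event.
; The event creates a player for the LS_RobotCofre sequence and plays it after a short delay.
; When it finishes, it sets DebeSeguir, destroys the sequence actor, then unhides BP_VEOTRES and enables its tick.
; A timeline that would bob the VEO component vertically is present but never runs.
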(event Custom|SalirDelCofre
  (bind (_outactor _returnvalue) (Sequencer|Player|CreateLevelSequencePlayer "/Game/Blueprints/LS_RobotCofre.LS_RobotCofre"))
  (Utilities|FlowControl|Delay 0.2)
  (EventDispatchers|AssignOnFinished _returnvalue (delegate Custom|OnFinished_Event))
  (Sequencer|Player|Play _returnvalue :!class /Script/MovieScene.MovieSceneSequencePlayer))

(event Custom|OnFinished_Event
  (Variables|Default|SetdebeSeguir true)
  (Actor|DestroyActor (stale Custom|SalirDelCofre _outactor))
  (bind _returnvalue (Actor|GetActorOfClass "/Game/Blueprints/BP_VEOTRES.BP_VEOTRES_C"))
  (Rendering|SetActorHiddenInGame _returnvalue false)
  (Actor|Tick|SetActorTickEnabled _returnvalue true))

(event Custom|cast)

(event Collision|EventActorBeginOverlap
  (params (OtherActor :type Actor%20Object%20Reference)))

(event EventBeginPlay)

(fn ConstructionScript)