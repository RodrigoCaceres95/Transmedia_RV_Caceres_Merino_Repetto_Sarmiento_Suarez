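; Cubicle door actor whose marble panel opens only after a linked chest has been opened.
; BeginPlay stores the closed relative position, and the Interactuar event checks that CofreRequerido is valid and opened.
; A timeline then lerps the mesh along local Z by AlturaApertura.
; The door opens once with no closing logic, and never opens without an assigned chest.
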(event EventInteractuar
  (params (Instigador :type Actor%20Object%20Reference))
  (bind _poscerrada (Variables|Default|GetPosCerrada))
  (bind _cofrerequerido (Variables|Default|GetCofreRequerido))
  (if (not (Variables|Default|GetbAbierta))
    (Utilities|IsValid _cofrerequerido
      (:Is%20Valid
        (if (Variables|/Game/Blueprints/BP_Cofre.BP_Cofre_C|GetbFueAbierto _cofrerequerido)
          (Variables|Default|SetbAbierta true)
          (bind _apertura (Timeline|TL%20Puerta Play)
            (:Update
              (Transformation|SetRelativeLocation (Variables|Default|GetSM_puerta_marmol) (Math|Vector|Lerp(Vector) _poscerrada (+ _poscerrada (Math|Vector|MakeVector 0.0 0.0 (Variables|Default|GetAlturaApertura))) _apertura) false false))))))))

(event Collision|EventActorBeginOverlap
  (params (OtherActor :type Actor%20Object%20Reference)))

(event EventTick
  (params (DeltaSeconds :type Float%20%28single-precision%29)))

(event EventBeginPlay
  (Variables|Default|SetPosCerrada (Variables|/Script/Engine.SceneComponent|GetRelativeLocation (Variables|Default|GetSM_puerta_marmol))))

(fn ConstructionScript)