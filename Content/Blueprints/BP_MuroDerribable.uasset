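; BP_MuroDerribable is an interactable wall actor that plays a knock-down Level Sequence, LS_DerriboPared, when triggered.
; Its Interactuar event uses a DoOnce to create a sequence player and play it a single time, with a debug print.
; Box overlap events show a Billboard while BP_ThirdPersonCharacter overlaps the actor and hide it when the character leaves, serving as a proximity indicator.
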(event OnComponentBeginOverlap(Box)
  (params (OverlappedComponent :type Primitive%20Component%20Object%20Reference) (OtherActor :type Actor%20Object%20Reference) (OtherComp :type Primitive%20Component%20Object%20Reference) (OtherBodyIndex :type Integer) (bFromSweep :type Boolean) (SweepResult :type Hit%20Result%20Structure%20%28by%20ref%29))
  (bind _asbp_third_person_character (Utilities|Casting|CastToBP_ThirdPersonCharacter OtherActor))
  (if (Collision|IsOverlappingActor _asbp_third_person_character :!class /Script/Engine.Actor)
    (Rendering|SetVisibility (Variables|Default|GetBillboard) true false)))

(event OnComponentEndOverlap(Box)
  (params (OverlappedComponent :type Primitive%20Component%20Object%20Reference) (OtherActor :type Actor%20Object%20Reference) (OtherComp :type Primitive%20Component%20Object%20Reference) (OtherBodyIndex :type Integer))
  (bind _asbp_third_person_character (Utilities|Casting|CastToBP_ThirdPersonCharacter OtherActor))
  (if (not (Collision|IsOverlappingActor _asbp_third_person_character :!class /Script/Engine.Actor))
    (Rendering|SetVisibility (Variables|Default|GetBillboard) false false)))

(event EventBeginPlay)

(event Collision|EventActorBeginOverlap
  (params (OtherActor :type Actor%20Object%20Reference)))

(event EventTick
  (params (DeltaSeconds :type Float%20%28single-precision%29)))

(event EventInteractuar
  (params (Instigador :type Actor%20Object%20Reference))
  (Utilities|FlowControl|DoOnce false
    (:Completed
      (bind _returnvalue (Sequencer|Player|CreateLevelSequencePlayer "/Game/Blueprints/LS_DerriboPared.LS_DerriboPared"))
      (Sequencer|Player|Play _returnvalue :!class /Script/MovieScene.MovieSceneSequencePlayer)
      (Development|PrintString "play"))))

(fn ConstructionScript)