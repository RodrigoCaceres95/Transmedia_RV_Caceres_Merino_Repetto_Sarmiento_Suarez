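; BP_Cofre is a chest actor that opens and closes its lid when interacted with.
; The Interactuar event prints a debug message and toggles the Abierto flag, playing or reversing the TLTapa timeline, and sets FueAbierto on opening.
; The timeline alpha lerps the lid mesh's roll rotation to swing it open or shut.
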(event EventBeginPlay)

(event Collision|EventActorBeginOverlap
  (params (OtherActor :type Actor%20Object%20Reference)))

(event EventTick
  (params (DeltaSeconds :type Float%20%28single-precision%29)))

(event EventInteractuar
  (params (Instigador :type Actor%20Object%20Reference))
  (Development|PrintString "interact recibido")
  (if (Variables|Default|GetbAbierto)
    (Variables|Default|SetbAbierto false)
    (bind _alpha (Timeline|TLTapa Reverse)
      (:Update
        (Transformation|SetRelativeRotation (Variables|Default|GetSM_tapa_cofre) (Math|Rotator|MakeRotator (Math|Float|Lerp 0.0 -75.0 _alpha) 0.0 0.0) false false)))
    (else
      (Variables|Default|SetbAbierto true)
      (Variables|Default|SetbFueAbierto true)
      (Timeline|TLTapa Play))))

(fn ConstructionScript)