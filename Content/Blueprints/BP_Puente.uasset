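; BP_Puente is a bridge actor that plays a raise sequence once, when triggered while a character is in its zone.
; Box overlap events set and clear the JugadorEnZona flag for any Character, without checking that it is the player.
; The SubirPuente event checks that flag, then a DoOnce creates and plays a LS_Puente Level Sequence player and prints a debug message.
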(event OnComponentBeginOverlap(Box)
  (params (OverlappedComponent :type Primitive%20Component%20Object%20Reference) (OtherActor :type Actor%20Object%20Reference) (OtherComp :type Primitive%20Component%20Object%20Reference) (OtherBodyIndex :type Integer) (bFromSweep :type Boolean) (SweepResult :type Hit%20Result%20Structure%20%28by%20ref%29))
  (Utilities|Casting|CastToCharacter OtherActor)
  (Variables|Default|SetbJugadorEnZona true))

(event OnComponentEndOverlap(Box)
  (params (OverlappedComponent :type Primitive%20Component%20Object%20Reference) (OtherActor :type Actor%20Object%20Reference) (OtherComp :type Primitive%20Component%20Object%20Reference) (OtherBodyIndex :type Integer))
  (Utilities|Casting|CastToCharacter OtherActor)
  (Variables|Default|SetbJugadorEnZona false))

(event Custom|SubirPuente
  (if (Variables|Default|GetbJugadorEnZona)
    (Utilities|FlowControl|DoOnce false
      (:Completed
        (bind _returnvalue (Sequencer|Player|CreateLevelSequencePlayer "/Game/Blueprints/LS_Puente.LS_Puente"))
        (Sequencer|Player|Play _returnvalue :!class /Script/MovieScene.MovieSceneSequencePlayer)
        (Development|PrintString "puente subido abz")))))

(event EventBeginPlay)

(event Collision|EventActorBeginOverlap
  (params (OtherActor :type Actor%20Object%20Reference)))

(event EventTick
  (params (DeltaSeconds :type Float%20%28single-precision%29)))

(fn ConstructionScript)