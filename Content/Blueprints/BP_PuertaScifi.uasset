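; BP_PuertaScifi is a keycard-locked sci-fi door with upper and lower panels that slide vertically apart.
; The Box overlap enables input for the third-person character, where E checks TieneTarjeta and prints a hint without the card.
; EstaAbierta toggles a Timeline between play and reverse, lerping panels from their BeginPlay positions; the flag reads inverted, turning false on opening.
; Unconnected TL_AbrirPuerta logic never runs.
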(event OnComponentBeginOverlap(Box)
  (params (OverlappedComponent :type Primitive%20Component%20Object%20Reference) (OtherActor :type Actor%20Object%20Reference) (OtherComp :type Primitive%20Component%20Object%20Reference) (OtherBodyIndex :type Integer) (bFromSweep :type Boolean) (SweepResult :type Hit%20Result%20Structure%20%28by%20ref%29))
  (Utilities|Casting|CastToBP_ThirdPersonCharacter OtherActor)
  (Input|EnableInput (Game|GetPlayerController 0)))

(event OnComponentEndOverlap(Box)
  (params (OverlappedComponent :type Primitive%20Component%20Object%20Reference) (OtherActor :type Actor%20Object%20Reference) (OtherComp :type Primitive%20Component%20Object%20Reference) (OtherBodyIndex :type Integer))
  (Utilities|Casting|CastToBP_ThirdPersonCharacter OtherActor)
  (Input|DisableInput (Game|GetPlayerController 0)))

(event EventBeginPlay
  (Variables|Default|SetPosInicialSup (Variables|/Script/Engine.SceneComponent|GetRelativeLocation (Variables|Default|GetPuertaSuperior)))
  (Variables|Default|SetPosInicialInf (Variables|/Script/Engine.SceneComponent|GetRelativeLocation (Variables|Default|GetPuertaInferior))))

(event Collision|EventActorBeginOverlap
  (params (OtherActor :type Actor%20Object%20Reference)))

(event EventTick
  (params (DeltaSeconds :type Float%20%28single-precision%29)))

(event Input|KeyboardEvents|E
  (params (Key :type Key%20Structure :default "None"))
  (bind _posinicialinf (Variables|Default|GetPosInicialInf))
  (bind _posinicialsup (Variables|Default|GetPosInicialSup))
  (:Pressed
    (bind _asbp_third_person_character (Utilities|Casting|CastToBP_ThirdPersonCharacter (Game|GetPlayerCharacter 0)))
    (if (Variables|/Game/ThirdPerson/Blueprints/BP_ThirdPersonCharacter.BP_ThirdPersonCharacter_C|GetTieneTarjeta _asbp_third_person_character)
      (if (Variables|Default|GetEstaAbierta)
        (Variables|Default|SetEstaAbierta false)
        (bind _progreso (Timeline|Timeline PlayFromStart)
          (:Update
            (Transformation|SetRelativeLocation (Variables|Default|GetPuertaSuperior) (Math|Vector|Lerp(Vector) _posinicialsup (+ _posinicialsup "0.000000,0.000000,150.000000") _progreso) false false)
            (Transformation|SetRelativeLocation (Variables|Default|GetPuertaInferior) (Math|Vector|Lerp(Vector) _posinicialinf (+ _posinicialinf "0.000000,0.000000,-150.000000") _progreso) false false)))
        (else
          (Variables|Default|SetEstaAbierta true)
          (Timeline|Timeline Reverse)))
      (else
        (Development|PrintString "\"Necesito buscar la tarjeta\"")))))

(fn ConstructionScript)